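; FeeblePathGameState is the game state that tracks which character, Wizard or Knight, each of the two players takes in multiplayer.
; TogglePlayerCharacterChoices swaps the two roles based on player one's current type, printing an error if it is neither.
; The RepNotify on P1CharacterType reaches the MultiplayerMenu through the game instance to toggle the displayed character images.
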(fn ConstructionScript)

(fn TogglePlayerCharacterChoices
  (if (== (Variables|Default|GetP1CharacterType) "/Game/Blueprints/PlayerCharacters/Wizard/Wizard.Wizard_C")
    (Variables|Default|SetP1CharacterType "/Game/Blueprints/PlayerCharacters/Knight/Knight.Knight_C")
    (Variables|Default|SetP2CharacterType "/Game/Blueprints/PlayerCharacters/Wizard/Wizard.Wizard_C")
    (return)
    (elif (== (Variables|Default|GetP1CharacterType) "/Game/Blueprints/PlayerCharacters/Knight/Knight.Knight_C")
      (Variables|Default|SetP1CharacterType "/Game/Blueprints/PlayerCharacters/Wizard/Wizard.Wizard_C")
      (Variables|Default|SetP2CharacterType "/Game/Blueprints/PlayerCharacters/Knight/Knight.Knight_C")
      (return)
      (else
        (Development|PrintString "Toggle player cast failed")))))

(fn OnRepP1CharacterType
  (bind _asfeeble_path_game_instance (Utilities|Casting|CastToFeeblePathGameInstance (Game|GetGameInstance)))
  (Default|TogglePlayerCharacterImages (Variables|/Game/Blueprints/FeeblePathGameInstance.FeeblePathGameInstance_C|GetMultiplayerMenu _asfeeble_path_game_instance))
  (return))