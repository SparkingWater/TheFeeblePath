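; FP_PlayerState is a player state Blueprint that puts the player UI and the game-over screen on screen for its owning player controller.
; On BeginPlay it re-checks every frame through a Delay loop until the controlled pawn is no longer a SpectatorPawn, then shows the cursor and adds Players_CommonUI.
; LoadGameOverUI clears all widgets and adds Game_over_u, without using its GameWasLost input.
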(event Custom|Load%20Player%20UI
  (bind _asplayer_controller (Utilities|Casting|CastToPlayerController (Components|GetOwner)))
  (Variables|/Script/Engine.PlayerController|SetbShowMouseCursor _asplayer_controller true)
  (bind _returnvalue (UserInterface|CreateWidget "/Game/Blueprints/PlayerCharacters/Players_CommonUI.Players_CommonUI_C" _asplayer_controller))
  (UserInterface|Viewport|AddtoViewport _returnvalue 0))

(event Custom|Load%20Game%20Over%20UI
  (params (Game%20Was%20Lost :type Boolean))
  (bind _asplayer_controller (Utilities|Casting|CastToPlayerController (Components|GetOwner)))
  (Viewport|RemoveAllWidgets)
  (bind _returnvalue (UserInterface|CreateWidget "/Game/Blueprints/PlayerCharacters/game_over_u.game_over_u_C" _asplayer_controller))
  (UserInterface|Viewport|AddtoViewport _returnvalue 0))

(event EventBeginPlay
  (bind _asplayer_controller (Utilities|Casting|CastToPlayerController (Components|GetOwner)))
  (if (== (Utilities|GetClass (Pawn|GetControlledPawn _asplayer_controller)) "/Script/Engine.SpectatorPawn") :!label _label
    (Utilities|FlowControl|Delay (Utilities|Time|GetWorldDeltaSeconds))
    (goto _label)
    (else
      (CallFunction|LoadPlayerUI))))

(fn ConstructionScript)