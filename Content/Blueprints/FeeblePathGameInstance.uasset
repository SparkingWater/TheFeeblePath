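; Game instance for Feeble Path that tracks logged-in players, each one's Wizard or Knight character class, and the current game state.
; It swaps the two class choices, spawns and possesses a pawn per player at given transforms, and clears players before opening the starting level on a new game.
; State handling is minimal: TransitionToState only handles leaving the multiplayer menu, and ShowMenu checks for Playing without acting on it.
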(event EventInit)

(fn TogglePlayerCharacterChoices
  (if (== (Variables|Default|GetP1CharacterType) "/Game/Blueprints/PlayerCharacters/Wizard/Wizard.Wizard_C")
    (Variables|Default|SetP1CharacterType "/Game/Blueprints/PlayerCharacters/Knight/Knight.Knight_C")
    (Variables|Default|SetP2CharacterType "/Game/Blueprints/PlayerCharacters/Wizard/Wizard.Wizard_C")
    (return)
    (elif (== (Variables|Default|GetP1CharacterType) "/Game/Blueprints/PlayerCharacters/Knight/Knight.Knight_C")
      (Variables|Default|SetP1CharacterType "/Game/Blueprints/PlayerCharacters/Wizard/Wizard.Wizard_C")
      (Variables|Default|SetP2CharacterType "/Game/Blueprints/PlayerCharacters/Knight/Knight.Knight_C")
      (return)
      (else
        (Development|PrintString "Toggle player cast failed")))))

(fn AddPlayer
  (params (NewPlayer :type Player%20Character%20Controller%20Object%20Reference))
  (Utilities|Array|Add (Variables|Default|GetPlayers) NewPlayer)
  (if (> (Utilities|Array|Length (Variables|Default|GetPlayers)) 2)
    (Development|PrintString "More than two players have logged in. This is unsupported" true true "(R=0.000000,G=0.660000,B=1.000000,A=1.000000)" 1e+01))
  (return))

(fn GetPlayer
  (params (PlayerNumber :type Integer))
  (return (Utilities|Array|Get(acopy) (Variables|Default|GetPlayers) (- PlayerNumber 1))))

(fn SpawnPlayersinLevel
  (params (P1Spawn :type Transform) (P2Spawn :type Transform))
  (if (< (Utilities|Array|Length (Variables|Default|GetPlayers)) 2)
    (Development|PrintString "Only one player active, are you testing?")
    (else
      (Utilities|FlowControl|Sequence
        (:then_0
          _)
        (:then_1
          (bind _returnvalue (Game|SpawnActorfromClass (Variables|Default|GetP2CharacterType) P2Spawn "Undefined" 0 0))
          (Pawn|Possess (Utilities|Array|Get(acopy) (Variables|Default|GetPlayers) 1) _returnvalue)
          (return)))))
  (bind _returnvalue_2 (Game|SpawnActorfromClass (Variables|Default|GetP1CharacterType) P1Spawn "Undefined" 0 0))
  (Pawn|Possess (Utilities|Array|Get(acopy) (Variables|Default|GetPlayers)) _returnvalue_2))

(fn StartNewGame
  (bind _asfeeble_path_game_instance (Utilities|Casting|CastToFeeblePathGameInstance (Game|GetGameInstance)))
  (Utilities|Array|Clear (Variables|FeeblePathGameInstance_C|GetPlayers _asfeeble_path_game_instance))
  (Game|OpenLevel(byName) (Variables|Default|GetStartingLevel))
  (return))

(fn ShowMenu
  (Utilities|IsCurrentState "NewEnumerator1"))