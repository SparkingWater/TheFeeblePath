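; Game mode for a two-player game that spawns a Wizard and a Knight and assigns them to the players.
; PostLogin collects player controllers; when the second joins, SpawnPlayersInLevel spawns both pawns at stored transforms and possesses them according to P1Type from the game instance.
; OnPlayerDeath loads the game-over UI through each player's state, while OnFeeblesSaved is empty.
; Older spawn logic using named PlayerStarts remains unconnected.
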(event Custom|On%20Player%20Death
  (for _array_element (Variables|Default|GetPlayers)
    (Default|LoadGameOverUI (.AsFP%20Player%20State (Utilities|Casting|CastToFP_PlayerState (Variables|/Script/Engine.Controller|GetPlayerState _array_element))) false)))

(event Custom|On%20Feebles%20Saved
  (params (Number%20of%20Feebles%20Saved :type Float%20%28single-precision%29)))

(event EventBeginPlay
  (bind _asfp_game_instance (Utilities|Casting|CastToFP_GameInstance (Game|GetGameInstance)))
  (Variables|Default|SetGameInstance _asfp_game_instance))

(event EventPostLogin
  (params (NewPlayer :type Player%20Controller%20Object%20Reference))
  (bind _asplayer_character_controller (Utilities|Casting|CastToPlayerCharacterController NewPlayer)
    (:then
      (Utilities|Array|Add (Variables|Default|GetPlayers) _asplayer_character_controller)
      (if (<= (Utilities|Array|Length (Variables|Default|GetPlayers)) 2)
        (if (== (Utilities|Array|Length (Variables|Default|GetPlayers)) 2)
          (CallFunction|SpawnPlayersinLevel))
        (else
          (Development|PrintString "More than two players have logged in" true true "(R=0.000000,G=0.660000,B=1.000000,A=1.000000)" 1e+01))))
    (:CastFailed
      (Development|PrintString "player cant be cast as character controller" true true "(R=0.000000,G=0.660000,B=1.000000,A=1.000000)" 2e+01))))

(fn ConstructionScript)

(fn SpawnPlayersinLevel
  (bind _returnvalue (Game|SpawnActorfromClass "/Game/Blueprints/PlayerCharacters/Wizard/Wizard.Wizard_C" (LocalVariables|GetWizard%20Start%20Transform) "Undefined" 0 0))
  (LocalVariables|SetWizardPawn _returnvalue)
  (bind _returnvalue_2 (Game|SpawnActorfromClass "/Game/Blueprints/PlayerCharacters/Knight/Knight.Knight_C" (LocalVariables|GetKnight%20Start%20Transform) "Undefined" 0 0))
  (LocalVariables|SetKnightPawn _returnvalue_2)
  (if (== (Variables|/Game/Blueprints/FP_GameInstance.FP_GameInstance_C|GetP1Type_ (Variables|Default|GetGameInstance)) "/Game/Blueprints/PlayerCharacters/Wizard/Wizard.Wizard_C")
    (Pawn|Possess (Utilities|Array|Get(acopy) (Variables|Default|GetPlayers)) (LocalVariables|GetWizardPawn))
    (Pawn|Possess (Utilities|Array|Get(acopy) (Variables|Default|GetPlayers) 1) (LocalVariables|GetKnightPawn))
    (else
      (Pawn|Possess (Utilities|Array|Get(acopy) (Variables|Default|GetPlayers)) (LocalVariables|GetKnightPawn))
      (Pawn|Possess (Utilities|Array|Get(acopy) (Variables|Default|GetPlayers) 1) (LocalVariables|GetWizardPawn)))))