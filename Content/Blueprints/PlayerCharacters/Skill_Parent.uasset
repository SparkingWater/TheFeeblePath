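; Base skill component that spawns a spell actor for a player character or fire spawner and tracks its cooldown and lifetime.
; UseSkill spawns the actor at the player's skills arrow and attaches it, or unhides a persistent one.
; Tick updates readiness and calls EndSkill on expiry, which hides or destroys the actor.
; Only zero-duration skills start their cooldown on use; EndSkill does not start it.
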(event EventBeginPlay
  (bind _successful (Skillstates|Initialize))
  (if (not _successful)
    (Development|PrintString "Error linking spell component")))

(event EventTick
  (params (DeltaSeconds :type Float%20%28single-precision%29))
  (Skillstates|UpdateSkill))

(fn TickCooldown
  (if (> (Variables|Cooldown|GetCurrent%20Cooldown) 0.0)
    (Variables|Cooldown|SetCurrent%20Cooldown (- (Variables|Cooldown|GetCurrent%20Cooldown) (Utilities|Time|GetWorldDeltaSeconds)))
    (return (<= (Variables|Cooldown|GetCurrent%20Cooldown) 0.0))
    (else
      (return true))))

(fn StartCooldown
  (Variables|Cooldown|SetCurrent%20Cooldown (Variables|Cooldown|GetSpellTotalCooldown)))

(fn UseSkill
  (params (MakeHiddenComponentVisible :type Boolean))
  (bind _spellactorcomponent (Variables|Components|GetSpellActorComponent))
  (bind _duration (Variables|Customproperties|GetDuration))
  (Variables|SpawningProperties|SetActorNeverDestroyed MakeHiddenComponentVisible)
  (Utilities|FlowControl|Sequence
    (:then_0
      ;[1 1 1] Spawn component or make it visible
      (if (and (Variables|SpawningProperties|GetActorNeverDestroyed) (!= _spellactorcomponent 0))
        (Rendering|SetActorHiddenInGame _spellactorcomponent false)
        (else
          (Skillactions|SpawnSkillComponent (Variables|Spawningproperties|GetSpawnedObjectType) (Transformation|GetWorldTransform (Variables|SpawningProperties|GetSpawn%20Location)) false))))
    (:then_1
      (if (!= _duration 0.0)
        (Variables|Customproperties|SetLifetimeLeft _duration)))
    (:then_3
      (Variables|GeneralProperties|SetIsSkillInUse true)
      (if (== (Variables|Customproperties|GetDuration) 0.0)
        (Cooldown|StartCooldown)))
    (:then_4
      (return true))))

(fn UpdateSkill
  (Utilities|FlowControl|Sequence
    (:then_0
      (bind _spellisready (Cooldown|TickCooldown))
      (Variables|GeneralProperties|SetIsReadyToUse _spellisready))
    (:then_1
      (if (Variables|GeneralProperties|GetIsSkillInUse)
        (if (> (Variables|Customproperties|GetDuration) 0.0)
          (bind _output_get (Variables|Customproperties|SetLifetimeLeft (- (Variables|Customproperties|GetLifetimeLeft) (Utilities|Time|GetWorldDeltaSeconds))))
          (if (< _output_get 0.0)
            (Skillstates|EndSkill true)))))))

(fn EndSkill
  (params (Expired :type Boolean))
  (Utilities|FlowControl|Sequence
    (:then_0
      (if (Variables|SpawningProperties|GetActorNeverDestroyed)
        (Rendering|SetActorHiddenInGame (Variables|Components|GetSpellActorComponent) true)
        (else
          (Actor|DestroyActor (Variables|Components|GetSpellActorComponent)))))
    (:then_1
      (Variables|GeneralProperties|SetIsSkillInUse false))))

(fn Initialize
  (bind _returnvalue (Components|GetOwner))
  (bind _asplayer_character (Utilities|Casting|CastToPlayerCharacter _returnvalue)
    (:then
      (bind _output_get (Variables|Components|SetSourcePlayer _asplayer_character))
      (Variables|SpawningProperties|SetSpawn%20Location (Variables|/Game/Blueprints/PlayerCharacters/PlayerCharacter.PlayerCharacter_C|GetSkillsArrowComponent _output_get))
      (bind _asplayer_character_controller (Utilities|Casting|CastToPlayerCharacterController (Pawn|GetController _output_get))
        (:then
          (Variables|Components|SetSourcePlayerController _asplayer_character_controller)
          (return true))
        (:CastFailed
          _)))
    (:CastFailed
      (bind _asi_fire_spawner (Utilities|Casting|CastToI_FireSpawner _returnvalue)
        (:then
          (Variables|Components|SetSourceNonPlayerObject _asi_fire_spawner)
          (return true))
        (:CastFailed
          _))))
  (return false))

(fn SpawnSkillComponent
  (params (ActorClass :type Actor%20Class%20Reference) (SpawnTransform :type Transform) (Hidden :type Boolean))
  (bind _returnvalue (Game|SpawnActorfromClass ActorClass SpawnTransform "AlwaysSpawn" 0 0))
  (bind _output_get (Variables|Components|SetSpellActorComponent _returnvalue))
  (Transformation|AttachActorToActor _output_get (Variables|Components|GetSourcePlayer) "None" "KeepWorld" "SnapToTarget" "KeepRelative" true)
  (Rendering|SetActorHiddenInGame (Variables|Components|GetSpellActorComponent) Hidden))