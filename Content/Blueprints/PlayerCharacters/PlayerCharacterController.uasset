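; Player controller Blueprint that handles click-style interaction with objects under the cursor.
; On Interact press it traces under the cursor on the Visibility channel and stores any InteractiveObject hit on the player character, otherwise printing a debug message.
; PositionCastingCursor is an unfinished stub that checks a skill-casting cursor flag but does nothing yet.
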(event Input|ActionEvents|InputActionInteract
  (params (Key :type Key%20Structure :default "AnyKey"))
  (:Pressed
    (bind _asinteractive_object (Utilities|Casting|CastToInteractiveObject (.hitactor (.HitResult (Game|Player|GetHitResultUnderCursorbyChannel "TraceTypeQuery1" true))))
      (:then
        (bind _asplayer_character (Utilities|Casting|CastToPlayerCharacter (Game|GetPlayerCharacter 0)))
        (Variables|/Game/Blueprints/PlayerCharacters/PlayerCharacter.PlayerCharacter_C|SetObjectInteractedWIth _asplayer_character _asinteractive_object))
      (:CastFailed
        (Development|PrintString "Not interactive")))))

(fn ConstructionScript)

(fn PositionCastingCursor
  (if (Variables|Default|GetShouldShowSkillCastingCursor)
    _))