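; I_Torch is a torch tile that can be switched on or off as part of a chain of triggerable objects.
; EventTriggerObject stores the incoming Fact in OnOff and shows or hides the Flame component to match.
; It then relays the same state to every entry in TriggeredObjects through their own EventTriggerObject.
; The construction script only runs the parent version.
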(event EventEventTriggerObject
  (params (Fact :type Boolean) (Index :type Integer) (Value :type Float%20%28single-precision%29))
  (bind _output_get (Variables|Default|SetOnOff Fact))
  (if _output_get
    (Rendering|SetVisibility (Variables|Default|GetFlame) true false)
    (else
      (Rendering|SetVisibility (Variables|Default|GetFlame) false false)))
  (for _array_element (Variables|Default|GetTriggered%20Objects)
    (Default|EventTriggerObject _array_element (Variables|Default|GetOnOff) 0 0.0)))

(fn ConstructionScript
  (|CallParentFunction))