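; Feeble character: an AI creature that walks along its forward vector while a Blackboard flag is set.
; A visibility sphere tracks noticed objects, while helper functions classify players by distance, step speed and direction, and set a mood material parameter.
; Dragging lifts the mesh on a timeline, dropping restores gravity, and damage or falling-object overlap can destroy it.
; BeginPlay is empty; Blackboard, player-data and speed setup are disconnected.
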(event OnComponentBeginOverlap(VisibilitySphere)
  (params (OverlappedComponent :type Primitive%20Component%20Object%20Reference) (OtherActor :type Actor%20Object%20Reference) (OtherComp :type Primitive%20Component%20Object%20Reference) (OtherBodyIndex :type Integer) (bFromSweep :type Boolean) (SweepResult :type Hit%20Result%20Structure%20%28by%20ref%29))
  ;[1 1 1] New Object in the Visibility Sphere
  (if (!= OtherActor self)
    (bind (_result _interestingobject) (CallFunction|IstheObjectNew OtherActor))
    (if _result
      (Utilities|Array|Add (Variables|General|GetNoticedObjects) _interestingobject))))

(event OnComponentEndOverlap(VisibilitySphere)
  (params (OverlappedComponent :type Primitive%20Component%20Object%20Reference) (OtherActor :type Actor%20Object%20Reference) (OtherComp :type Primitive%20Component%20Object%20Reference) (OtherBodyIndex :type Integer))
  ;[1 1 1] Object is now out of Visibility Sphere
  (bind _interestingobject (CallFunction|IstheObjectNew OtherActor))
  (if (not (Utilities|Enum|Equal(Enum) (.InterestingObject (Utilities|Struct|BreakFeeble_InterestingObjects _interestingobject)) "NewEnumerator4"))
    (Utilities|Array|RemoveItem (Variables|General|GetNoticedObjects) _interestingobject)))

(event Custom|OnDraggingStarted
  (params (CasterZPosition :type Float%20%28single-precision%29))
  (Variables|WizardHandskill|SetLiftingOffset (Variables|/Script/Engine.SceneComponent|GetRelativeLocation (Variables|Character|GetMesh)))
  (Variables|WizardHandskill|SetTimelineFinished false)
  (Variables|WizardHandskill|SetZLiftingAmount (+ 1e+02 (- CasterZPosition (.z (Transformation|GetActorLocation)))))
  (Variables|/Script/Engine.CharacterMovementComponent|SetGravityScale (Variables|Character|GetCharacterMovement) 0.0)
  (Variables|WizardHandskill|SetEarlyDnDDrop false)
  (bind _feeble_z_position (Timeline|Timeline_0 PlayFromStart)
    (:Update
      (if (Variables|WizardHandskill|GetEarlyDnDDrop)
        (Timeline|Timeline_0 Stop)
        (else
          (Transformation|SetRelativeLocation (Variables|Character|GetMesh) (+ (Variables|WizardHandskill|GetLiftingOffset) (Math|Vector|MakeVector 0.0 0.0 (* _feeble_z_position (Variables|WizardHandskill|GetZLiftingAmount)))) true false))))
    (:Finished
      (Variables|WizardHandskill|SetTimelineFinished true))))

(event Custom|OnDrop
  (Variables|/Script/Engine.CharacterMovementComponent|SetGravityScale (Variables|Character|GetCharacterMovement) 1e+02)
  (Transformation|SetActorLocation (+ (Transformation|GetActorLocation) (Math|Vector|MakeVector 0.0 0.0 (Variables|WizardHandskill|GetZLiftingAmount))) false true)
  (Transformation|SetRelativeLocation (Variables|Character|GetMesh) (Variables|WizardHandskill|GetLiftingOffset) true false))

(event EventTick
  (params (DeltaSeconds :type Float%20%28single-precision%29))
  ;[1 1 1] Tick
  (if (ScalableFloat|GetValueasBool (Variables|Default|GetBlackboard) (Variables|Default|GetHasActiveGoald_BBFieldName))
    (Pawn|Input|AddMovementInput (Variables|MovementDirection|GetFeebleForwardVector) 1.0 false)
    (else
      (Components|Movement|StopMovementImmediately (Variables|Character|GetCharacterMovement)))))

(event Game|Damage|EventAnyDamage
  (params (Damage :type Float%20%28single-precision%29) (DamageType :type Damage%20Type%20Object%20Reference) (InstigatedBy :type Controller%20Object%20Reference) (DamageCauser :type Actor%20Object%20Reference))
  ;[1 1 1] Apply damage to Feeble
  (Development|PrintString (Utilities|String|Append (Utilities|String|ToString(Float) (Variables|Default|GetHealth)) " feeble health "))
  (bind _output_get (Variables|Default|SetHealth (- (Variables|Default|GetHealth) Damage)))
  (if (<= _output_get 0.0)
    (Actor|DestroyActor)))

(event Collision|EventActorBeginOverlap
  (params (OtherActor :type Actor%20Object%20Reference))
  ;[1 1 1] Killing feebles upon rock collision
  (bind _asi_falling_object (Utilities|Casting|CastToI_FallingObject OtherActor))
  (if (Utilities|Enum|Equal(Enum) (Variables|/Game/Blueprints/Tiles/FeeblePathActor.FeeblePathActor_C|GetObjectType _asi_falling_object) "NewEnumerator5")
    (Actor|DestroyActor)))

(event EventBeginPlay
  ;[1 1 1] BeginPlay
)

(fn ConstructionScript
  (|CallParentFunction)
  (bind _returnvalue (Rendering|Material|CreateDynamicMaterialInstance (Variables|Character|GetMesh) 3 "/Game/Geometry/Meshes/3rd_iteration/pasted__lambert13.pasted__lambert13" :!class /Script/Engine.PrimitiveComponent))
  (bind _output_get (Variables|Default|SetMoodRelatedMaterial _returnvalue))
  (Rendering|Material|SetScalarParameterValue _returnvalue "Mood" 0.0 :!class /Script/Engine.MaterialInstanceDynamic))

(fn CalculateDistancetotheClosestPlayer
  (params (MinDetectionRange :type Float%20%28single-precision%29) (MaxDetectionRange :type Float%20%28single-precision%29))
  (bind _outactors (Actor|GetAllActorsOfClass "/Game/Blueprints/PlayerCharacters/PlayerCharacter.PlayerCharacter_C"))
  (for _array_element _outactors
    (bind (_distance _direction) (CallFunction|CalculateDistancetothePoint (Transformation|GetActorLocation _array_element)))
    (if (< _distance (LocalVariables|GetDist))
      (if (and (< _distance MaxDetectionRange) (> _distance MinDetectionRange))
        (bind _returnvalue (Collision|LineTraceByChannel (Transformation|GetActorLocation _array_element) (Transformation|GetActorLocation) "TraceTypeQuery1" false (Utilities|Array|MakeArray _array_element) "None"))
        (if (not _returnvalue)
          (LocalVariables|SetDist _distance)
          (LocalVariables|SetClosestPlayer _array_element)
          (LocalVariables|SetFeebleDirection _direction)))))
  (return (LocalVariables|GetDist) (LocalVariables|GetClosestPlayer) (/ (LocalVariables|GetFeebleDirection) (LocalVariables|GetDist))))

(fn IstheObjectNew
  (params (Object :type Actor%20Object%20Reference))
  (Utilities|FlowControl|Sequence
    (:then_0
      (bind _asthird_person_character (Utilities|Casting|CastToThirdPersonCharacter Object)
        (:then
          (LocalVariables|SetObjectType (Variables|/Game/Blueprints/PlayerCharacters/ThirdPersonCharacter.ThirdPersonCharacter_C|GetFeeblePathObjectType _asthird_person_character)))
        (:CastFailed
          (bind _asfeeble_path_actor (Utilities|Casting|CastToFeeblePathActor Object)
            (:then
              (LocalVariables|SetObjectType (Variables|/Game/Blueprints/Tiles/FeeblePathActor.FeeblePathActor_C|GetObjectType _asfeeble_path_actor)))
            (:CastFailed
              (LocalVariables|SetObjectType "NewEnumerator4"))))))
    (:then_1
      (if (Utilities|Enum|Equal(Enum) (LocalVariables|GetObjectType) "NewEnumerator4")
        (return false "")))
    (:then_2
      (for _array_element (Variables|General|GetNoticedObjects)
        (if (and (== (.ActorReference (Utilities|Struct|BreakFeeble_InterestingObjects _array_element)) Object) (Utilities|Enum|NotEqual(Enum) (.InterestingObject (Utilities|Struct|BreakFeeble_InterestingObjects _array_element)) "NewEnumerator4"))
          (return false _array_element)))
      (return true (Utilities|Struct|MakeFeeble_InterestingObjects (LocalVariables|GetObjectType) Object false)))))

(fn HandleSpeedChange
  (bind _charactermovement (Variables|Character|GetCharacterMovement))
  (bind _charactermovement_2 (Variables|Character|GetCharacterMovement))
  (Utilities|FlowControl|Sequence
    (:then_0
      ;[1 1 1] Acceleration
      (if (Utilities|Enum|Equal(Enum) (Variables|Movementproperties|GetFeeble_SpeedState) "NewEnumerator1")
        (if (Math|Float|NearlyEqual(Float) (Class|MovementComponent|GetMaxSpeed (Variables|Character|GetCharacterMovement)) (Variables|MovementProperties|GetMaxSpeed) 1.0)
          (Variables|Movementproperties|SetFeeble_SpeedState "NewEnumerator0")
          (else
            (Variables|/Script/Engine.CharacterMovementComponent|SetMaxWalkSpeed _charactermovement_2 (+ (Class|MovementComponent|GetMaxSpeed _charactermovement_2) (Variables|MovementProperties|GetAccelerationStep)))))))
    (:then_1
      ;[1 1 1] Acceleration
      (if (Utilities|Enum|Equal(Enum) (Variables|Movementproperties|GetFeeble_SpeedState) "NewEnumerator2")
        (if (Math|Float|NearlyEqual(Float) (Class|MovementComponent|GetMaxSpeed (Variables|Character|GetCharacterMovement)) 0.0 1.0)
          (Variables|Movementproperties|SetFeeble_SpeedState "NewEnumerator0")
          (else
            (Variables|/Script/Engine.CharacterMovementComponent|SetMaxWalkSpeed _charactermovement (- (Class|MovementComponent|GetMaxSpeed _charactermovement) (Variables|MovementProperties|GetAccelerationStep)))))))
    (:then_2
      (if (Math|Vector|NotEqual(Vector) (Variables|MovementDirection|GetDirectionChangeStep) "0, 0, 0" 0.0001)
        (CallFunction|InterpolateDirection)))))

(fn InterpolateDirection
  (if (Math|Vector|NotEqual(Vector) (Variables|MovementDirection|GetFeebleForwardVector) (Variables|MovementDirection|GetDesiredForwardVector) 0.0001)
    (Variables|MovementDirection|SetFeebleForwardVector (+ (Variables|MovementDirection|GetFeebleForwardVector) (Variables|MovementDirection|GetDirectionChangeStep)))
    (else
      (Variables|MovementDirection|SetDirectionChangeStep "0, 0, 0"))))

(fn PrintChecksMessage
  (params (Message :type String))
  (Development|PrintString Message false true "(R=0.320000,G=0.000000,B=0.277667,A=1.000000)"))

(fn PrintDirectionPickingMessage
  (params (Message :type String))
  (Development|PrintString Message false true "(R=0.000000,G=0.033377,B=0.720000,A=1.000000)"))

(fn UpdatePlayerData
  (params (Index :type Integer))
  (bind _playersdata (Variables|Playerinteraction|GetPlayersData))
  (bind _item (Utilities|Array|Get(acopy) _playersdata Index))
  (bind (_distance _direction _isvisible) (CallFunction|CalculateDistancetothePoint (Transformation|GetActorLocation (.playeractor _item))))
  (LocalVariables|SetDistance _distance)
  (LocalVariables|SetVisible _isvisible)
  (if (< (LocalVariables|GetDistance) (Variables|Playerinteraction|GetPlayerFarRange))
    (if (> (LocalVariables|GetDistance) (Variables|Playerinteraction|GetPlayerCloseRange))
      (return (Utilities|Struct|MakeFeeble_PlayerData (.playeractor _item) "NewEnumerator2" (LocalVariables|GetVisible) (LocalVariables|GetDistance)))
      (else
        (return (Utilities|Struct|MakeFeeble_PlayerData (.playeractor _item) "NewEnumerator1" (LocalVariables|GetVisible) (LocalVariables|GetDistance)))))
    (else
      (return (Utilities|Struct|MakeFeeble_PlayerData (.playeractor _item) "NewEnumerator0" (LocalVariables|GetVisible) (LocalVariables|GetDistance))))))

(fn AdjustMood
  (params (MoodFloat :type Float%20%28single-precision%29))
  (Rendering|Material|SetScalarParameterValue (Variables|Default|GetMoodRelatedMaterial) "Mood" MoodFloat :!class /Script/Engine.MaterialInstanceDynamic))