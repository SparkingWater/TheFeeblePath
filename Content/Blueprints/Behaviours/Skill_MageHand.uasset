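; Mage Hand skill component for the Wizard that handles choosing, dragging and dropping a Feeble.
; On BeginPlay it caches the Wizard and its controller, and choosing enables dragging only when the hand cooldown is near zero.
; StartDragging saves and overrides the Feeble's movement type, shows its effect sphere and registers it on the Wizard.
; Drop restores both and restarts the cooldown; Grab is an empty stub.
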(event EventBeginPlay
  ;[1 1 1] Setup
  (bind _aswizard (Utilities|Casting|CastToWizard (Components|GetOwner)))
  (bind _output_get (Variables|Default|SetWizard _aswizard))
  (bind _aswizard_controller (Utilities|Casting|CastToWizardController (Pawn|GetController _output_get)))
  (Variables|Default|SetInput _aswizard_controller))

(fn Grab
  (params (Object%20Under%20Mouse :type Actor%20Object%20Reference))
  (if (not false)
    (if (> 0.0 0.0)
      _)))

(fn EnableChoosingFeeble
  (if (Math|Float|NearlyEqual(Float) (Variables|/Game/Blueprints/Characters/PlayerCharacters/Wizard.Wizard_C|GetHand_CurrentCooldown (Variables|Default|GetWizard)) 0.0 0.02)
    (Variables|Default|SetDraggingEnabled true)))

(fn StartDragging
  (params (Victim :type Feeble%20Character%20Object%20Reference))
  (Variables|Default|SetFeeble Victim)
  (Variables|Default|SetMovementType (Variables|/Game/Blueprints/Characters/Feebles/FeebleCharacter.FeebleCharacter_C|GetFeebleMovementType (Variables|Default|GetFeeble)))
  (Variables|/Game/Blueprints/Characters/Feebles/FeebleCharacter.FeebleCharacter_C|SetFeebleMovementType (Variables|Default|GetFeeble) "NewEnumerator4")
  (Development|SetHiddeninGame (Variables|/Game/Blueprints/Characters/Feebles/FeebleCharacter.FeebleCharacter_C|GetDraggingEffectSphere (Variables|Default|GetFeeble)) false false)
  (Rendering|SetVisibility (Variables|/Game/Blueprints/Characters/Feebles/FeebleCharacter.FeebleCharacter_C|GetDraggingEffectSphere (Variables|Default|GetFeeble)) true false)
  (Variables|Default|SetIsDraggingFeeble true)
  (Variables|/Game/Blueprints/Characters/PlayerCharacters/PlayerCharacter.PlayerCharacter_C|SetDraggedFeeble (Variables|Default|GetWizard) (Variables|Default|GetFeeble)))

(fn Drop
  (bind _feeble (Variables|Default|GetFeeble))
  (bind _wizard (Variables|Default|GetWizard))
  (bind _draggingeffectsphere (Variables|/Game/Blueprints/Characters/Feebles/FeebleCharacter.FeebleCharacter_C|GetDraggingEffectSphere _feeble))
  (Variables|Default|SetDraggingEnabled false)
  (Variables|Default|SetIsDraggingFeeble false)
  (Variables|/Game/Blueprints/Characters/Feebles/FeebleCharacter.FeebleCharacter_C|SetFeebleMovementType (Variables|Default|GetFeeble) (Variables|Default|GetMovementType))
  (Development|SetHiddeninGame _draggingeffectsphere true false)
  (Rendering|SetVisibility _draggingeffectsphere false false)
  (Variables|/Game/Blueprints/Characters/PlayerCharacters/Wizard.Wizard_C|SetHand_CurrentCooldown _wizard (Variables|/Game/Blueprints/Characters/PlayerCharacters/Wizard.Wizard_C|GetHand_Cooldown _wizard)))