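; Skill_Fireball is a fireball skill behaviour that launches a Fireball projectile from a given transform.
; Fire spawns the Fireball actor, then passes it velocity, lifetime, damage, size and explosion radius through SetValues.
; Speed derives from despawn distance over despawn time, and direction is the negated right vector of the projectile's Fireball component.
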(fn Fire
  (params (Spawn%20Location :type Transform))
  (bind _returnvalue (Game|SpawnActorfromClass "/Game/Blueprints/Objects/Fireball.Fireball_C" Spawn%20Location "Undefined" 0 0))
  (Default|SetValues _returnvalue (* (/ (* (Math|Vector|GetRightVector (Variables|/Game/Blueprints/Objects/Fireball.Fireball_C|GetFireball _returnvalue)) (Variables|Default|GetDistance%20Before%20Despawn)) (Variables|Default|GetTime%20Before%20Despawn)) -1.0) (Variables|Default|GetTime%20Before%20Despawn) (Variables|Default|GetDamage) (Variables|Default|GetSize%20of%20Fireball) (Variables|Default|GetExplosion%20Size)))