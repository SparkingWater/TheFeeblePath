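; Skill_Parent is a base skill Blueprint that gives a player skill cooldown handling.
; On BeginPlay it casts its owner to PlayerCharacter and caches that character along with its FeeblePath player controller.
; StartCooldown disables the skill and loads the wait time into a remaining-time counter.
; Tick counts this down by world delta seconds, re-enabling the skill on a tick that finds it at zero or below.
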(event EventBeginPlay
  (bind _asplayer_character (Utilities|Casting|CastToPlayerCharacter (Components|GetOwner)))
  (bind _output_get (Variables|Default|SetMy%20Player%20Character _asplayer_character))
  (bind _asfeeble_path_player_controller (Utilities|Casting|CastToFeeblePathPlayerController (Pawn|GetController _output_get)))
  (Variables|Default|SetMy%20Player%20Controller _asfeeble_path_player_controller))

(event EventTick
  (params (DeltaSeconds :type Float%20%28single-precision%29))
  (CallFunction|TickCooldown))

(fn TickCooldown
  (if (<= (Variables|Default|GetCurrent%20Cooldown%20Remaining) 0.0)
    (Variables|Default|SetIs%20Skill%20Enabled true)
    (else
      (Variables|Default|SetCurrent%20Cooldown%20Remaining (- (Variables|Default|GetCurrent%20Cooldown%20Remaining) (Utilities|Time|GetWorldDeltaSeconds))))))

(fn StartCooldown
  (Variables|Default|SetCurrent%20Cooldown%20Remaining (Variables|Default|GetCooldown%20Time%20To%20Wait))
  (Variables|Default|SetIs%20Skill%20Enabled false))