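; Mage shield skill for a Wizard owner that spawns and removes a protective shield actor, gated by energy and exhaustion.
; Shield spawns a MageShield snapped to the Wizard when energy remains and exhaustion is clear; Release destroys it.
; While shielded, Tick releases and exhausts when energy minus delta is non-negative, without decrementing energy.
; Otherwise, energy recharges per tick, unscaled by delta, and exhaustion clears at the cap.
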(event EventTick
  (params (DeltaSeconds :type Float%20%28single-precision%29))
  (if (Variables|Default|GetIs%20Shielded)
    (if (>= (- (Variables|Default|GetShield%20Energy) (Utilities|Time|GetWorldDeltaSeconds)) 0.0) ; Check for exhaustion
      ;[1 1 1] Exhaust if run out of energy
      (CallFunction|Release)
      (Variables|Default|SetIs%20Exhausted true))
    (else
      ;[1 1 1] Recharge energy
      (if (< (+ (Variables|Default|GetShield%20Energy) (Variables|Default|GetEnergy%20Recovery%20Rate%20%28sec%29)) (Variables|Default|GetMax%20Energy%20%28sec%29))
        (Variables|Default|SetShield%20Energy (+ (Variables|Default|GetShield%20Energy) (Variables|Default|GetEnergy%20Recovery%20Rate%20%28sec%29)))
        (else
          (Variables|Default|SetShield%20Energy (Variables|Default|GetMax%20Energy%20%28sec%29))
          (Variables|Default|SetIs%20Exhausted false) ; After energy fully refilled, remove exhaustion
        )))))

(event EventBeginPlay
  ;[1 1 1] Setup
  (bind _aswizard (Utilities|Casting|CastToWizard (Components|GetOwner)))
  (Variables|Default|SetWizard _aswizard))

(fn Shield
  (params (Spawn%20Location :type Transform))
  (if (not (Variables|Default|GetIs%20Exhausted))
    (if (> (Variables|Default|GetShield%20Energy) 0.0)
      (Variables|Default|SetIs%20Shielded true)
      (bind _returnvalue (Game|SpawnActorfromClass "/Game/Blueprints/Objects/MageShield.MageShield_C" Spawn%20Location "Undefined" 0 0))
      (bind _output_get (Variables|Default|SetCurrent%20Shield _returnvalue))
      (Transformation|AttachActorToActor _output_get (Variables|Default|GetWizard) "None" "SnapToTarget" "SnapToTarget" "KeepRelative" true))))

(fn Release
  (Variables|Default|SetIs%20Shielded false)
  (Actor|DestroyActor (Variables|Default|GetCurrent%20Shield)))