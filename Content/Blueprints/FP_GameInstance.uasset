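; Game instance that manages LAN multiplayer sessions and the multiplayer menu.
; Host, search, join and destroy events wrap session nodes with debug prints; hosting opens Pablo_Level as a listen server.
; SEARCHGame travels by console open command with the given IP, while SearchOnly just stores results, whose first entry JOINGame uses.
; A CurrentFrame state machine creates, shows and hides the menu widget; StartNewGameOLD is unwired.
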(event Custom|HOSTGame
  (bind _returnvalue (Game|GetPlayerController 0))
  ;[1 1 1] Host Game
  (|Session _returnvalue 0 true
    (:OnSuccess
      (bind _asfp_game_mode (Utilities|Casting|CastToFP_GameMode (Game|GetGameMode)))
      (Development|ExecuteConsoleCommand "open Pablo_Level?listen" _returnvalue)
      (Development|PrintString "Session created"))
    (:OnFailure
      (Development|PrintString "Session create error"))))

(event Custom|SEARCHGame
  (params (IP :type String))
  ;[1 1 1] Search Games
  (bind _results (|FindSessions (Game|GetPlayerController 0) 1 true)
    (:OnSuccess
      (Variables|Default|SetSessionResults _results)
      (Development|PrintString "SUCCESS Sessions found" true true "(R=0.000000,G=0.660000,B=1.000000,A=1.000000)" 2.0)
      (Development|ExecuteConsoleCommand (Utilities|String|Append "open " IP)))
    (:OnFailure
      (Development|PrintString "FAILED to find sessions" true true "(R=0.000000,G=0.660000,B=1.000000,A=1.000000)" 2.0))))

(event Custom|DESTROYGame
  ;[1 1 1] Destroy Game
  (|DestroySession (Game|GetPlayerController 0)
    (:OnSuccess
      (Development|PrintString "Succesfully destroyed session"))
    (:OnFailure
      (Development|PrintString "Session destroy error"))))

(event Custom|JOINGame
  ;[1 1 1] Join Game
  (|JoinSession (Game|GetPlayerController 0) (Utilities|Array|Get(acopy) (Variables|Default|GetSessionResults))
    (:OnSuccess
      (Development|PrintString "Succesfully joined to session" true true "(R=0.000000,G=0.660000,B=1.000000,A=1.000000)" 2.0))
    (:OnFailure
      (Development|PrintString "Session join error" true true "(R=0.000000,G=0.660000,B=1.000000,A=1.000000)" 2.0))))

(event Custom|Search%20Only
  (params (IP :type String))
  (Development|PrintString "searching")
  (bind _results (|FindSessions (Game|GetPlayerController 0) 1 true)
    (:OnSuccess
      (Variables|Default|SetSessionResults _results)
      (Development|PrintString "SUCCESS Sessions found" true true "(R=0.000000,G=0.660000,B=1.000000,A=1.000000)" 2.0))
    (:OnFailure
      (Development|PrintString "FAILED to find sessions" true true "(R=0.000000,G=0.660000,B=1.000000,A=1.000000)" 2.0))))

(fn StartNewGameOLD)

(fn ShowMenu
  (Utilities|IsCurrentFrame "NewEnumerator0"
    (:True
      (CallFunction|LoadMenus)
      (Utilities|TransitiontoFrame "NewEnumerator2"
        (:%20
          _)))
    (:False
      _))
  (switch Utilities|FlowControl|Switch|SwitchonFrameStates (Variables|Default|GetCurrentFrame)
    (:NewEnumerator0
      _)
    (:NewEnumerator1
      _)
    (:NewEnumerator2
      (UserInterface|Viewport|AddtoViewport (Variables|Default|GetMultiplayerMenu) 0)
      (Variables|/Script/Engine.PlayerController|SetbShowMouseCursor (Game|GetPlayerController 0) true)))
  (return))

(fn LoadMenus
  (bind _returnvalue (UserInterface|CreateWidget "/Game/Blueprints/MultiplayMenu.MultiplayMenu_C"))
  (Variables|Default|SetMultiplayerMenu _returnvalue)
  (return))

(fn OnRepGameHasBeenLost)