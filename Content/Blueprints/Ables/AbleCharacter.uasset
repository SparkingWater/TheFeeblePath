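; Able character that takes damage, can be picked up, dropped and slapped, and is destroyed when health runs out.
; Dragging disables gravity and uses a timeline to raise only the mesh, by an amount based on the caster's height, stopping if flagged for early drop.
; Dropping teleports the actor up by that full amount, resets the mesh offset and applies strong gravity.
; A slap only sets a flag and logs.
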(event Custom|OnDraggingStarted
  (params (CasterZPosition :type Float%20%28single-precision%29))
  (Variables|Default|SetLiftingOffset (Variables|/Script/Engine.SceneComponent|GetRelativeLocation (Variables|Character|GetMesh)))
  (Variables|Default|SetTimelineFinished false)
  (Variables|Default|SetZLiftingAmount (+ 1e+02 (- CasterZPosition (.z (Transformation|GetActorLocation)))))
  (Variables|/Script/Engine.CharacterMovementComponent|SetGravityScale (Variables|Character|GetCharacterMovement) 0.0)
  (Variables|Default|SetEarlyDnDDrop false)
  (bind _feeble_z_position (Timeline|Timeline_0 PlayFromStart)
    (:Update
      (if (Variables|Default|GetEarlyDnDDrop)
        (Timeline|Timeline_0 Stop)
        (else
          (Transformation|SetRelativeLocation (Variables|Character|GetMesh) (+ (Variables|Default|GetLiftingOffset) (Math|Vector|MakeVector 0.0 0.0 (* _feeble_z_position (Variables|Default|GetZLiftingAmount)))) true false))))
    (:Finished
      (Variables|Default|SetTimelineFinished true))))

(event Custom|OnSlap
  (Variables|Default|SetGotSlapped true)
  (Development|PrintString "SLAP!" false))

(event Custom|OnDrop
  (Variables|/Script/Engine.CharacterMovementComponent|SetGravityScale (Variables|Character|GetCharacterMovement) 1e+02)
  (Transformation|SetActorLocation (+ (Transformation|GetActorLocation) (Math|Vector|MakeVector 0.0 0.0 (Variables|Default|GetZLiftingAmount))) false true)
  (Transformation|SetRelativeLocation (Variables|Character|GetMesh) (Variables|Default|GetLiftingOffset) true false))

(event Game|Damage|EventAnyDamage
  (params (Damage :type Float%20%28single-precision%29) (DamageType :type Damage%20Type%20Object%20Reference) (InstigatedBy :type Controller%20Object%20Reference) (DamageCauser :type Actor%20Object%20Reference))
  (bind _output_get (Variables|Default|SetHealth (- (Variables|Default|GetHealth) Damage)))
  (Development|PrintString (Utilities|String|Append "Able Health: " (Utilities|String|ToString(Float) _output_get)) false)
  (if (<= _output_get 0.0)
    (Actor|DestroyActor)))

(fn ConstructionScript
  (|CallParentFunction))