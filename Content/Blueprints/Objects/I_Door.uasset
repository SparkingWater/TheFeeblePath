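; A triggerable door that slides its static mesh vertically between closed and open positions.
; TriggerObject sets IsActive only on the authority, and its RepNotify plays or reverses the OpenDoor timeline.
; The timeline offsets the mesh from its starting world location by a height scaled by its curve.
; Doors flagged IsOpenAtStart set the timeline to its end time on BeginPlay to pop open.
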(event EventBeginPlay
  (Variables|Default|SetInitial%20Location (Transformation|GetWorldLocation (Variables|Default|GetStaticMesh)))
  (if (Variables|Default|GetIsOpenAtStart)
    (bind _output_get (Variables|Default|SetTime%20overide 1.0)) ; Set the door animation to final frame so it 'pops' to that position
    ;[1 1 1] Animate door opening
    (bind _dooropening (Timeline|Open%20door SetNewTime)
      (:Update
        (Transformation|SetWorldLocation (Variables|Default|GetStaticMesh) (+ (Variables|Default|GetInitial%20Location) (Math|Vector|MakeVector 0.0 0.0 (* _dooropening (Variables|Default|GetHeight%20To%20Move)))) false false)))))

(event EventOnRepIsActive
  ;[1 1 1] Animate door opening
  (if (Variables|Default|GetIsActive_)
    (bind _dooropening (Timeline|Open%20door Play)
      (:Update
        (Transformation|SetWorldLocation (Variables|Default|GetStaticMesh) (+ (Variables|Default|GetInitial%20Location) (Math|Vector|MakeVector 0.0 0.0 (* _dooropening (Variables|Default|GetHeight%20To%20Move)))) false false)))
    (else
      (Timeline|Open%20door Reverse))))

(event EventTriggerObject
  (params (Active :type Boolean) (Index :type Integer) (Value :type Float%20%28single-precision%29))
  (Networking|SwitchHasAuthority
    (:Authority
      (Variables|Default|SetIsActive_ Active))))

(fn ConstructionScript
  (|CallParentFunction))