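; Lever actor that toggles between active and inactive when the player character begins overlapping it.
; Each toggle calls EventTriggerObject on every object in TriggeredObjects, passing the new state as Fact.
; A timeline plays or reverses to swing the handle, offsetting the pitch from the rotation stored at BeginPlay.
; The toggle runs through the lever's own EventTriggerObject event, which ignores incoming arguments.
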(event Collision|EventActorBeginOverlap
  (params (OtherActor :type Actor%20Object%20Reference))
  (Utilities|Casting|CastToPlayerCharacter OtherActor)
  (CallFunction|EventTriggerObject false 0 0.0))

(event EventBeginPlay
  (Variables|Default|SetInitial%20Rotation (Transformation|GetWorldRotation (Variables|Default|GetLever%20Handle))))

(event EventEventTriggerObject
  (params (Fact :type Boolean) (Index :type Integer) (Value :type Float%20%28single-precision%29))
  (bind _initial_rotation (Variables|Default|GetInitial%20Rotation))
  (Variables|Default|SetIsInActivePosition (not (Variables|Default|GetIsInActivePosition)))
  (for _array_element (Variables|Default|GetTriggered%20Objects)
    (Default|EventTriggerObject _array_element (Variables|Default|GetIsInActivePosition) 0 0.0))
  (if (Variables|Default|GetIsInActivePosition)
    (bind _lever_rotation (Timeline|Lever%20Handle%20Animation Play)
      (:Update
        (Transformation|SetWorldRotation (Variables|Default|GetLever%20Handle) (Math|Rotator|MakeRotator (.roll _initial_rotation) (+ _lever_rotation (.pitch (Variables|Default|GetInitial%20Rotation))) (.yaw _initial_rotation)) false false)))
    (else
      (Timeline|Lever%20Handle%20Animation Reverse))))

(fn ConstructionScript
  (|CallParentFunction))