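; Falling rocks object that turns loose when triggered.
; The EventTriggerObject event switches on physics simulation for three Rock components and three StaticMesh components at once.
; It holds no other logic: the construction script only calls its parent, and nothing in the file resets the pieces.
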(event EventEventTriggerObject
  (params (Fact :type Boolean) (Index :type Integer) (Value :type Float%20%28single-precision%29))
  (Physics|SetSimulatePhysics (Variables|Default|GetRock1) true)
  (Physics|SetSimulatePhysics (Variables|Default|GetRock2) true)
  (Physics|SetSimulatePhysics (Variables|Default|GetRock3) true)
  (Physics|SetSimulatePhysics (Variables|Default|GetStaticMesh1) true)
  (Physics|SetSimulatePhysics (Variables|Default|GetStaticMesh2) true)
  (Physics|SetSimulatePhysics (Variables|Default|GetStaticMesh3) true))

(fn ConstructionScript
  (|CallParentFunction))