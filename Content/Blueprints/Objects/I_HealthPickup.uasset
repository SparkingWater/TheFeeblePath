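; Health pickup actor that heals a PlayerCharacter on overlap and respawns after a delay.
; The server-authority branch of the overlap event calls RestoreHealth on the character with the configured healing amount.
; It then hides the actor and disables mesh collision, restoring visibility and query-only collision once the respawn delay ends, so the same actor is reused.
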(event Collision|EventActorBeginOverlap
  (params (OtherActor :type Actor%20Object%20Reference))
  (Networking|SwitchHasAuthority
    (:Authority
      (bind _asplayer_character (Utilities|Casting|CastToPlayerCharacter OtherActor))
      (Default|RestoreHealth _asplayer_character (Variables|Default|GetHealing%20Amount))
      (Collision|SetCollisionEnabled (Variables|Default|GetStaticMesh) "NoCollision")
      (Rendering|SetActorHiddenInGame true)
      (Utilities|FlowControl|Delay (Variables|Default|GetRespawn%20Delay))
      (Collision|SetCollisionEnabled (Variables|Default|GetStaticMesh) "QueryOnly")
      (Rendering|SetActorHiddenInGame false))))

(fn ConstructionScript
  (|CallParentFunction))