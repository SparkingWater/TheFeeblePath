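; Weight-triggered button that activates connected objects when enough ThirdPersonCharacter weight stands on it.
; The server adds and subtracts character weight on overlap, setting IsActive against the required threshold.
; Its OnRep handler triggers connected objects, plays a sound and moves the button with a timeline, reversed on release.
; Sticky switches ignore deactivation in that handler, so they stay pressed.
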(event EventBeginPlay
  (Variables|Default|SetInitial%20Location (Transformation|GetWorldLocation (Variables|Default|GetButton))))

(event EventOnRepIsActive
  (bind _returnvalue (Transformation|GetActorLocation))
  (if (Variables|Default|GetIs%20Sticky%20Switch)
    (if (Variables|Default|GetIsActive_)
      (CallFunction|TriggerConnectedObjects (Variables|Default|GetIsActive_) 0 0.0 :!label _label)
      ;[1 1 1] Animate the button & play sound
      (if (Variables|Default|GetIsActive_)
        (Audio|PlaySoundatLocation "/Game/sounds_and_music/Button.Button" _returnvalue)
        (bind _button_height (Timeline|Timeline_0 Play)
          (:Update
            (Transformation|SetWorldLocation (Variables|Default|GetButton) (+ (Variables|Default|GetInitial%20Location) (Math|Vector|MakeVector 0.0 0.0 _button_height)) true false)))
        (else
          (Audio|PlaySoundatLocation "/Game/sounds_and_music/Button.Button" _returnvalue)
          (Timeline|Timeline_0 Reverse))))
    (else
      (goto _label))))

(event Collision|EventActorBeginOverlap
  (params (OtherActor :type Actor%20Object%20Reference))
  (Networking|SwitchHasAuthority
    (:Authority
      (bind _asthird_person_character (Utilities|Casting|CastToThirdPersonCharacter OtherActor))
      (Variables|Default|SetTotal%20Weight%20on%20Button (+ (Variables|Default|GetTotal%20Weight%20on%20Button) (Variables|/Game/Blueprints/PlayerCharacters/ThirdPersonCharacter.ThirdPersonCharacter_C|GetWeight _asthird_person_character)))
      (Variables|Default|SetIsActive_ (>= (Variables|Default|GetTotal%20Weight%20on%20Button) (Variables|Default|GetWeight%20Needed%20to%20Trigger))) ; Doesnt need to trigger self so set active directly
    )))

(event Collision|EventActorEndOverlap
  (params (OtherActor :type Actor%20Object%20Reference))
  (Networking|SwitchHasAuthority
    (:Authority
      (bind _asthird_person_character (Utilities|Casting|CastToThirdPersonCharacter OtherActor))
      (Variables|Default|SetTotal%20Weight%20on%20Button (- (Variables|Default|GetTotal%20Weight%20on%20Button) (Variables|/Game/Blueprints/PlayerCharacters/ThirdPersonCharacter.ThirdPersonCharacter_C|GetWeight _asthird_person_character)))
      (Variables|Default|SetIsActive_ (>= (Variables|Default|GetTotal%20Weight%20on%20Button) (Variables|Default|GetWeight%20Needed%20to%20Trigger))) ; Doesnt need to trigger self so set active directly
    )))

(fn ConstructionScript
  (|CallParentFunction))