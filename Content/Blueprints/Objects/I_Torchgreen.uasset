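; I_Torchgreen is a triggerable torch object that lights when hit by fire damage and can activate other objects connected to it.
; Fire damage on an unlit torch calls TriggerObject to set it active.
; The IsActive replication notify then passes the state to connected objects and shows or hides the Fire component.
; On BeginPlay, ShouldStartLit sets only the flame's initial visibility.
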(event EventBeginPlay
  ;[1 1 1] Set torch flame on or off at start
  (Rendering|SetVisibility (Variables|Default|GetFire) (Variables|Default|GetShould%20Start%20Lit) true))

(event Game|Damage|EventAnyDamage
  (params (Damage :type Float%20%28single-precision%29) (DamageType :type Damage%20Type%20Object%20Reference) (InstigatedBy :type Controller%20Object%20Reference) (DamageCauser :type Actor%20Object%20Reference))
  ;[1 1 1] Light torch when hit with fire
  (Utilities|Casting|CastToFireDamage DamageType)
  (if (not (Variables|Default|GetIsActive_))
    (CallFunction|TriggerObject true 0 0.0)))

(event EventOnRepIsActive
  ;[1 1 1] When triggered, trigger connected objects and light / put out torch
  (CallFunction|TriggerConnectedObjects (Variables|Default|GetIsActive_) 0 0.0)
  (Rendering|SetVisibility (Variables|Default|GetFire) (Variables|Default|GetIsActive_) true))

(fn ConstructionScript
  (|CallParentFunction))