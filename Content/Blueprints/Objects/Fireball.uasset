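; Fireball projectile actor that explodes on impact, with speed, lifetime, size, damage and caster configured through SetValues.
; Hit spawns an I_FireExplosion at the mesh and destroys the actor, while a server-only timer from BeginPlay destroys it silently when Lifetime expires.
; The older overlap logic for direct damage, friendly-fire filtering by object type and fire-spawner effects is disconnected, and MoveForwards is not called here.
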(event Custom|End%20Fireball
  (Actor|DestroyActor))

(event EventBeginPlay
  (Networking|SwitchHasAuthority
    (:Authority
      (Utilities|FlowControl|Delay (Utilities|Time|GetWorldDeltaSeconds))
      (Utilities|FlowControl|Delay (Variables|Default|GetLifetime))
      (CallFunction|EndFireball))))

(event Collision|EventActorBeginOverlap
  (params (OtherActor :type Actor%20Object%20Reference)))

(event Collision|EventHit
  (params (MyComp :type Primitive%20Component%20Object%20Reference) (Other :type Actor%20Object%20Reference) (OtherComp :type Primitive%20Component%20Object%20Reference) (bSelfMoved :type Boolean) (HitLocation :type Vector :default "0, 0, 0") (HitNormal :type Vector :default "0, 0, 0") (NormalImpulse :type Vector :default "0, 0, 0") (Hit :type Hit%20Result%20Structure%20%28by%20ref%29))
  (bind _staticmesh (Variables|Default|GetStaticMesh))
  (bind _returnvalue (Transformation|GetWorldTransform _staticmesh))
  (Game|SpawnActorfromClass "/Game/Blueprints/Objects/I_FireExplosion.I_FireExplosion_C" (Math|Transform|MakeTransform (.location _returnvalue) (.rotation _returnvalue) "1,1,1") "Undefined" 0 0) ; Spawn spell explosion
  (CallFunction|EndFireball))

(fn ConstructionScript)

(fn SetValues
  (params (Speed :type Float%20%28single-precision%29) (Lifetime :type Float%20%28single-precision%29) (Size :type Float%20%28single-precision%29) (Damage :type Float%20%28single-precision%29) (Explosion%20Radius :type Float%20%28single-precision%29) (Was%20Cast%20By%20Player :type Boolean) (Caster :type Actor%20Object%20Reference))
  (bind _projectilemovement (Variables|Default|GetProjectileMovement))
  (bind _output_get (Variables|/Script/Engine.ProjectileMovementComponent|SetInitialSpeed _projectilemovement Speed))
  (Variables|/Script/Engine.ProjectileMovementComponent|SetMaxSpeed _projectilemovement _output_get)
  (Variables|Default|SetLifetime Lifetime)
  (Variables|Default|SetSize Size)
  (Transformation|SetWorldScale3D (Variables|Default|GetFireball_emmiter) (* "1.000000,1.000000,1.000000" (Variables|Default|GetSize)))
  (Variables|Default|SetDamage Damage)
  (Variables|Default|SetExplosion%20Radius Explosion%20Radius)
  (Variables|Default|SetWas%20Cast%20By%20Player Was%20Cast%20By%20Player)
  (Variables|Default|SetMy%20Owner Caster))

(fn MoveForwards
  (Transformation|SetActorLocation (+ (Transformation|GetActorLocation) (* (Transformation|GetActorForwardVector) (* (Variables|Default|GetSpeed) (Utilities|Time|GetWorldDeltaSeconds)))) true false)
  (return))

(fn PrintWhatWasHit
  (params (Should%20Print :type Boolean) (Feeble%20Path%20Actor%20Hit :type Feeble%20Path%20Actor%20Object%20Reference))
  (if Should%20Print
    (switch Utilities|FlowControl|Switch|SwitchonFeeblePath_ObjectTypes (Variables|/Game/Blueprints/Tiles/FeeblePathActor.FeeblePathActor_C|GetObjectType Feeble%20Path%20Actor%20Hit) ; Check what the fireball has hit
      (:NewEnumerator4
        ;[1 1 1] Print to log what object was hit
        (Development|PrintString (Utilities|String|Append (Utilities|String|MakeLiteralString "Fireball hit ") (Utilities|GetDisplayName Feeble%20Path%20Actor%20Hit)) :!label _label))
      (:NewEnumerator0
        (if (Variables|Default|GetWas%20Cast%20By%20Player)
          (Development|PrintString "Player's fireball hit a player. Ignoring")
          (else
            (Development|PrintString "Enemy fireball hit a player"))))
      (:NewEnumerator3
        (if (Variables|Default|GetWas%20Cast%20By%20Player)
          (Development|PrintString "Player's fireball hit a player. Ignoring")
          (else
            (Development|PrintString "Fireball hit feeble"))))
      (:NewEnumerator1
        (goto _label))
      (:NewEnumerator2
        (return))
      (:NewEnumerator5
        (return))
      (:NewEnumerator6
        (Development|PrintString "Fireball hit burnable"))
      (:NewEnumerator7
        (Development|PrintString "Fireball hit shield"))
      (:NewEnumerator8
        (if (Variables|Default|GetWas%20Cast%20By%20Player)
          (Development|PrintString "Fireball hit monster")
          (else
            (Development|PrintString "Enemy fireball hit a monster. Ignoring"))))
      (:NewEnumerator9
        (return)))
    (return)
    (else
      (return))))