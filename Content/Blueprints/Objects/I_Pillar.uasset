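; Pillar object whose top section tips over when triggered or when it takes fire damage.
; It caches the top's relative rotation and location at BeginPlay.
; EventTriggerObject plays a timeline that pitches the top toward MaxAngle and shifts it along X and Z by the two disposition modifiers, relative to those cached values.
; AnyDamage calls the same trigger only when the damage type casts to FireDamage.
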(event EventBeginPlay
  (bind _pillar_top (Variables|Default|GetPillar%20Top))
  (Variables|Default|SetPillarAngleOffset (Variables|/Script/Engine.SceneComponent|GetRelativeRotation _pillar_top))
  (Variables|Default|SetPillarLocationOffset (Variables|/Script/Engine.SceneComponent|GetRelativeLocation _pillar_top)))

(event Game|Damage|EventAnyDamage
  (params (Damage :type Float%20%28single-precision%29) (DamageType :type Damage%20Type%20Object%20Reference) (InstigatedBy :type Controller%20Object%20Reference) (DamageCauser :type Actor%20Object%20Reference))
  (Utilities|Casting|CastToFireDamage DamageType)
  (CallFunction|EventTriggerObject false 0 0.0))

(event EventEventTriggerObject
  (params (Fact :type Boolean) (Index :type Integer) (Value :type Float%20%28single-precision%29))
  (bind _pillar_top (Variables|Default|GetPillar%20Top))
  (bind _newtrack_0 (Timeline|Timeline_0 Play)
    (:Update
      (Transformation|SetRelativeRotation _pillar_top (Math|Rotator|CombineRotators (Math|Rotator|MakeRotator 0.0 (* _newtrack_0 (Variables|Default|GetMaxAngle)) 0.0) (Variables|Default|GetPillarAngleOffset)) false false)
      (Transformation|SetRelativeLocation _pillar_top (+ (Variables|Default|GetPillarLocationOffset) (Math|Vector|MakeVector (* _newtrack_0 (Variables|Default|GetDownwards_DispositionModifier)) 0.0 (* _newtrack_0 (Variables|Default|GetForward_DispositionModifier)))) false false))))

(fn ConstructionScript
  (|CallParentFunction))