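; InteractiveObject is a networked base Blueprint for objects that players can interact with and that can trigger other connected objects.
; The server tracks player characters entering and leaving its overlap, exposing a range check.
; TriggerConnectedObjects forwards active, index and value to linked objects, whose TriggerObject event stores them server-side in variables with RepNotify stubs.
; OnInteractClickInput and the RepNotifies are empty, with click behavior left to specific implementations.
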(event Custom|Event%20TriggerObject
  (params (Active :type Boolean) (Index :type Integer) (Value :type Float%20%28single-precision%29))
  (Networking|SwitchHasAuthority
    (:Authority
      (Variables|Default|SetIsActive_ Active)
      (Variables|Default|SetIndex_ Index)
      (Variables|Default|SetValue_ Value))))

(event Custom|OnInteractClickInput)

(event Collision|EventActorBeginOverlap
  (params (OtherActor :type Actor%20Object%20Reference))
  (Networking|SwitchHasAuthority
    (:Authority
      (bind _asplayer_character (Utilities|Casting|CastToPlayerCharacter OtherActor))
      (Utilities|Array|Add (Variables|Default|GetPlayersInRange) _asplayer_character)
      (Development|PrintString "Player entered interactive"))))

(event Collision|EventActorEndOverlap
  (params (OtherActor :type Actor%20Object%20Reference))
  (Networking|SwitchHasAuthority
    (:Authority
      (bind _asplayer_character (Utilities|Casting|CastToPlayerCharacter OtherActor))
      (Utilities|Array|RemoveItem (Variables|Default|GetPlayersInRange) _asplayer_character)
      (Development|PrintString "Player left interactive"))))

(fn ConstructionScript
  (|CallParentFunction))

(fn TriggerConnectedObjects
  (params (Active :type Boolean) (Index :type Integer) (Value :type Float%20%28single-precision%29))
  (Networking|SwitchHasAuthority ; Only run this on the server
    (:Authority
      (if (> (Utilities|Array|Length (Variables|Default|GetConnectedObjectsToTrigger)) 0)
        (for _array_element (Variables|Default|GetConnectedObjectsToTrigger)
          (CallFunction|EventTriggerObject _array_element Active Index Value))))
    (:Remote
      _))
  (return))

(fn IsPlayerinRange
  (params (Player :type Player%20Character%20Object%20Reference))
  (return (Utilities|Array|ContainsItem (Variables|Default|GetPlayersInRange) Player)))

(fn OnRepIsActive)

(fn OnRepIndex)

(fn OnRepValue)