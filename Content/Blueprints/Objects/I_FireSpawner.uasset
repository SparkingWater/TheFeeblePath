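; Fire spawner object that repeatedly launches fireballs on its own by driving a SkillFireball skill.
; On BeginPlay it copies its own fireball settings, such as class, speed, size, lifetime and cooldown, into the skill.
; Tick calls UseSkill every frame with no conditions, so any pacing between shots is left to the skill.
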(event EventBeginPlay
  (Variables|/Game/Blueprints/PlayerCharacters/AbstractVersion/Skill_Parent_Abs.Skill_Parent_Abs_C|SetSpellTotalCooldown (Variables|Default|GetSkill_Fireball) (Variables|Default|GetFireball%20Cooldown))
  (Variables|/Game/Blueprints/PlayerCharacters/AbstractVersion/Skill_Fireball_Abs.Skill_Fireball_Abs_C|SetSpeed (Variables|Default|GetSkill_Fireball) (Variables|Default|GetFireballSpeed))
  (Variables|/Game/Blueprints/PlayerCharacters/AbstractVersion/Skill_Parent_Abs.Skill_Parent_Abs_C|SetSpawnedObjectType (Variables|Default|GetSkill_Fireball) (Variables|Default|GetFireballClass))
  (Variables|/Game/Blueprints/PlayerCharacters/AbstractVersion/Skill_Parent_Abs.Skill_Parent_Abs_C|SetSpellComponent_Size (Variables|Default|GetSkill_Fireball) (Variables|Default|GetFireballSize))
  (Variables|/Game/Blueprints/PlayerCharacters/AbstractVersion/Skill_Parent_Abs.Skill_Parent_Abs_C|SetDuration (Variables|Default|GetSkill_Fireball) (Variables|Default|GetMaxLifetime)))

(event EventTick
  (params (DeltaSeconds :type Float%20%28single-precision%29))
  (Default|UseSkill (Variables|Default|GetSkill_Fireball) false))

(fn ConstructionScript
  (|CallParentFunction))