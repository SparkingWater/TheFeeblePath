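; Falling hazard object that can damage player characters, with its static mesh dropped through physics simulation by TriggerObject.
; BeginPlay stores the start location and calls TriggerObject with Active false, though the handler enables physics without checking any arguments.
; Server-only hit handling filters characters by two FeeblePathObjectType values.
; Damage and self-destruction run only if AlreadyDealtDamage is already true, and the flag is set only inside that branch.
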(event EventBeginPlay
  (Variables|Default|SetInitial%20Location (Transformation|GetActorLocation))
  (CallFunction|TriggerObject false 0 0.0))

(event EventTriggerObject
  (params (Active :type Boolean) (Index :type Integer) (Value :type Float%20%28single-precision%29))
  (Physics|SetSimulatePhysics (Variables|Default|GetStaticMesh) true))

(event Collision|EventHit
  (params (MyComp :type Primitive%20Component%20Object%20Reference) (Other :type Actor%20Object%20Reference) (OtherComp :type Primitive%20Component%20Object%20Reference) (bSelfMoved :type Boolean) (HitLocation :type Vector :default "0, 0, 0") (HitNormal :type Vector :default "0, 0, 0") (NormalImpulse :type Vector :default "0, 0, 0") (Hit :type Hit%20Result%20Structure%20%28by%20ref%29))
  (Networking|SwitchHasAuthority
    (:Authority
      (bind _asthird_person_character (Utilities|Casting|CastToThirdPersonCharacter Other))
      (if (or (Utilities|Enum|Equal(Enum) (Variables|/Game/Blueprints/PlayerCharacters/ThirdPersonCharacter.ThirdPersonCharacter_C|GetFeeblePathObjectType _asthird_person_character) "NewEnumerator0") (Utilities|Enum|Equal(Enum) (Variables|/Game/Blueprints/PlayerCharacters/ThirdPersonCharacter.ThirdPersonCharacter_C|GetFeeblePathObjectType _asthird_person_character) "NewEnumerator3"))
        (if (Variables|Default|GetAlreadyDealtDamage)
          (Game|Damage|ApplyDamage _asthird_person_character 1.0 0 0)
          (Variables|Default|SetAlreadyDealtDamage true)
          (Actor|DestroyActor))))))

(fn ConstructionScript
  (|CallParentFunction))