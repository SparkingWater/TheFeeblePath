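; Networked spike trap actor that periodically rises from and retracts to its starting position, damaging characters that touch it.
; The SpikeCycle timeline's event track alternates show and hide while IsActive is set, driving the ActivateSpikes timeline forward or backward to offset the actor's Z.
; The IsActive RepNotify restarts the cycle through a branch fixed to true, leaving its hide path unreachable.
; Box overlaps apply damage to FeebleCharacter or ThirdPersonCharacter on the authority only.
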(event OnComponentBeginOverlap(Box)
  (params (OverlappedComponent :type Primitive%20Component%20Object%20Reference) (OtherActor :type Actor%20Object%20Reference) (OtherComp :type Primitive%20Component%20Object%20Reference) (OtherBodyIndex :type Integer) (bFromSweep :type Boolean) (SweepResult :type Hit%20Result%20Structure%20%28by%20ref%29))
  (Networking|SwitchHasAuthority
    (:Authority
      (bind _asfeeble_character (Utilities|Casting|CastToFeebleCharacter OtherActor)
        (:then
          (Game|Damage|ApplyDamage _asfeeble_character 1.0 0 0))
        (:CastFailed
          (bind _asthird_person_character (Utilities|Casting|CastToThirdPersonCharacter OtherActor))
          (Game|Damage|ApplyDamage _asthird_person_character 1.0 0 0))))))

(event Custom|Show%20Spikes
  (bind _initial_location (Variables|Default|GetInitial%20Location))
  ;[1 1 1] Smooth movement of spikes
  (bind _spikes_z_position (Timeline|Activate%20Spikes Play)
    (:Update
      (Transformation|SetActorLocation (Math|Vector|MakeVector (.x _initial_location) (.y _initial_location) (+ (.z _initial_location) _spikes_z_position)) false false))))

(event Custom|Run%20Spike%20Cycle
  ;[1 1 1] Show and hide spikes
  (Timeline|Spike%20cycle%20:%29 Play
    (:Event%20Track
      (if (Variables|Default|GetIsActive_)
        (if (Variables|Default|GetSpikesOn)
          (CallFunction|ShowSpikes)
          (else
            (CallFunction|HideSpikes)))
        (Variables|Default|SetSpikesOn (not (Variables|Default|GetSpikesOn)))
        (else
          (Timeline|Spike%20cycle%20:%29 Stop))))))

(event Custom|Hide%20Spikes
  (bind _initial_location (Variables|Default|GetInitial%20Location))
  ;[1 1 1] Smooth movement of spikes
  (bind _spikes_z_position (Timeline|Activate%20Spikes Reverse)
    (:Update
      (Transformation|SetActorLocation (Math|Vector|MakeVector (.x _initial_location) (.y _initial_location) (+ (.z _initial_location) _spikes_z_position)) false false))))

(event EventBeginPlay
  ;[1 1 1] Save initial spike position
  (Variables|Default|SetInitial%20Location (Transformation|GetActorLocation))
  (CallFunction|RunSpikeCycle))

(event EventOnRepIsActive
  (if true
    (CallFunction|RunSpikeCycle)
    (else
      (CallFunction|HideSpikes))))

(fn ConstructionScript
  (|CallParentFunction))