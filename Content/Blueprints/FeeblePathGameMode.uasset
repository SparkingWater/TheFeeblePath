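; FeeblePathGameMode is a two-player game mode that tracks logged-in players and spawns their characters.
; PostLogin stores each PlayerCharacterController, printing a warning beyond two players.
; SpawnPlayersInLevel runs on authority, spawning and possessing the pawn classes held in the GameInstance at P1/P2 player starts, swapped when P1 is Wizard.
; With fewer than two players it spawns only P1; an older, disconnected copy of this spawn logic remains.
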(event EventBeginPlay
  (bind _asfeeble_path_game_instance (Utilities|Casting|CastToFeeblePathGameInstance (Game|GetGameInstance)))
  (Variables|Default|SetGameInstance _asfeeble_path_game_instance))

(event EventPostLogin
  (params (NewPlayer :type Player%20Controller%20Object%20Reference))
  (bind _asplayer_character_controller (Utilities|Casting|CastToPlayerCharacterController NewPlayer)
    (:then
      (Utilities|Array|Add (Variables|Default|GetPlayers) _asplayer_character_controller)
      (if (> (Utilities|Array|Length (Variables|Default|GetPlayers)) 2)
        (Development|PrintString "More than two players have logged in" true true "(R=0.000000,G=0.660000,B=1.000000,A=1.000000)" 1e+01)))
    (:CastFailed
      (Development|PrintString "player cant be cast as character controller" true true "(R=0.000000,G=0.660000,B=1.000000,A=1.000000)" 2e+01))))

(fn ConstructionScript)

(fn SpawnPlayersinLevel
  (bind _returnvalue (Class|GameModeBase|FindPlayerStart 0 "P2"))
  (bind _returnvalue_2 (Class|GameModeBase|FindPlayerStart 0 "P1"))
  (bind _returnvalue_3 (Transformation|GetActorTransform _returnvalue))
  (bind _returnvalue_4 (Transformation|GetActorTransform _returnvalue_2))
  (Networking|SwitchHasAuthority
    (:Authority
      (if (== (Variables|/Game/Blueprints/FeeblePathGameInstance.FeeblePathGameInstance_C|GetP1Type_ (Variables|Default|GetGameInstance)) "/Game/Blueprints/PlayerCharacters/Wizard/Wizard.Wizard_C")
        ;[1 1 1] Not sure why these have to be logically backwards but it works...
        (LocalVariables|SetP1%20Start%20Transform _returnvalue_3)
        (LocalVariables|SetP2%20Start%20Transform _returnvalue_4)
        (else
          (LocalVariables|SetP2%20Start%20Transform _returnvalue_3)
          (LocalVariables|SetP1%20Start%20Transform _returnvalue_4)))
      (if (< (Utilities|Array|Length (Variables|Default|GetPlayers)) 2)
        (Development|PrintString "Only one player active, are you testing?" true true "(R=0.000000,G=0.660000,B=1.000000,A=1.000000)" 2.0)
        (else
          (bind _returnvalue_5 (Game|SpawnActorfromClass (Variables|/Game/Blueprints/FeeblePathGameInstance.FeeblePathGameInstance_C|GetP2Type_ (Variables|Default|GetGameInstance)) (LocalVariables|GetP2%20Start%20Transform) "Undefined" 0 0))
          (Pawn|Possess (Utilities|Array|Get(acopy) (Variables|Default|GetPlayers) 1) _returnvalue_5)))
      (bind _returnvalue_6 (Game|SpawnActorfromClass (Variables|/Game/Blueprints/FeeblePathGameInstance.FeeblePathGameInstance_C|GetP1Type_ (Variables|Default|GetGameInstance)) (LocalVariables|GetP1%20Start%20Transform) "Undefined" 0 0))
      (Pawn|Possess (Utilities|Array|Get(acopy) (Variables|Default|GetPlayers)) _returnvalue_6)
      (return))))